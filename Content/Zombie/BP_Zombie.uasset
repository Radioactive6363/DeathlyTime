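; Zombie character that takes damage, dies once its health runs out and removes itself from the level.
; IsDamagable subtracts damage from Vida, then triggers a one-time death guarded by EstaVivo.
; Death detaches the controller, plays an animation, disables capsule collision, switches to ragdoll after a short delay, then destroys the actor on a timer.
; PlayZombieAMontage plays a random numbered montage section and returns the average section duration.
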(event `/Game/Blueprints/BPI_Damage.IsDamagable`
  (params (Damage :type "Float (double-precision)") (ImpactLocation :type "Vector Structure"))
  (`|ExecutionSequence`
    (:`then_0`
      (`self.DañoRecibido` Damage))
    (:`then_1`
      (if (<= (`self.Vida`) 0.0)
        (`self.ZombieNeutralizado`)))))

(event `DañoRecibido`
  (params (`DañoRecibido` :type "Float (double-precision)"))
  ; Eliminacion de Vida
  (set `self.Vida` (- (`self.Vida`) `DañoRecibido`)))

(event `ZombieNeutralizado`
  ; Comment
  (if (`self.EstaVivo?`)
    (`self.DetachFromControllerPendingDestroy`)
    (set `self.EstaVivo?` false)
    (`KismetSystemLibrary.PrintString` (`KismetStringLibrary.Concat_StrStr` (`KismetSystemLibrary.GetDisplayName` self) " Fui Destruido!") true true (struct :`R` 1.0 :`B` 0.012164 :`A` 1.0))
    (`SkeletalMeshComponent.PlayAnimation` (`self.Mesh`) (`self.New Anim to Play`) false)
    (`PrimitiveComponent.SetCollisionEnabled` (`self.CapsuleComponent`) "NoCollision")
    (`KismetSystemLibrary.Delay` 0.5)
    (`PrimitiveComponent.SetSimulatePhysics` (`self.Mesh`) true)
    (`KismetSystemLibrary.K2_SetTimer` null "DestruirZombie" 5.0)))

(event `DestruirZombie`
  (`self.K2_DestroyActor`))

(fn `PlayZombieAMontage`
  (params (AnimationMontage :type "AnimMontage Object Reference") (MontageName :type String))
  (returns (AnimationDuration :type "Float (double-precision)"))
  (bind _returnvalue (`AnimMontage.GetNumSections` AnimationMontage))
  (bind _returnvalue_2 (`self.PlayAnimMontage` AnimationMontage 1.0 (`KismetStringLibrary.Conv_StringToName` (`KismetStringLibrary.Concat_StrStr` MontageName (`KismetStringLibrary.Conv_IntToString` (`KismetMathLibrary.RandomIntegerInRange` 1 _returnvalue))))))
  (return (/ _returnvalue_2 _returnvalue)))

(fn `UserConstructionScript`)
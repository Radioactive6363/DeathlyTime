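; BP_Zombie is a damageable zombie actor that loses health and ragdolls on death.
; IsDamagable subtracts damage from Vida with debug prints, then calls ZombieNeutralizado once health reaches zero or below.
; Death enables mesh physics, applies an impulse along the actor's forward vector at the bone closest to the impact, and disables capsule collision.
; A timer then destroys the actor after a short delay.
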(event `/Game/Blueprints/BPI_Damage.IsDamagable`
  (params (Damage :type "Float (double-precision)") (ImpactLocation :type "Vector Structure"))
  (`|ExecutionSequence`
    (:`then_0`
      (`self.DañoRecibido` Damage))
    (:`then_1`
      (if (<= (`self.Vida`) 0.0)
        (`self.ZombieNeutralizado` ImpactLocation)))))

(event `DañoRecibido`
  (params (`DañoRecibido` :type "Float (double-precision)"))
  ; Eliminacion de Vida
  (bind _output_get (set `self.Vida` (- (`self.Vida`) `DañoRecibido`)))
  (`KismetSystemLibrary.PrintString` (`KismetStringLibrary.Concat_StrStr` (`KismetSystemLibrary.GetDisplayName` "BP_Zombie") "Tengo:" (`KismetStringLibrary.Conv_DoubleToString` _output_get) " de vida") true true (struct :`R` 0.259266 :`G` 1.0 :`A` 1.0))
  (`KismetSystemLibrary.PrintString` (`KismetStringLibrary.Concat_StrStr` "Recibi: " (`KismetStringLibrary.Conv_DoubleToString` `DañoRecibido`) " de daño!") true true (struct :`R` 1.0 :`G` 0.48018 :`A` 1.0)))

(event `ZombieNeutralizado`
  (params (ImpactoFinalLoc :type "Vector Structure"))
  (bind _mesh (`self.Mesh`))
  ; Comment
  (set `self.EstaVivo?` false)
  (`KismetSystemLibrary.PrintString` (`KismetStringLibrary.Concat_StrStr` (`KismetSystemLibrary.GetDisplayName` self) " Fui Destruido!") true true (struct :`R` 1.0 :`B` 0.012164 :`A` 1.0))
  (`PrimitiveComponent.SetSimulatePhysics` _mesh true)
  (`PrimitiveComponent.AddImpulse` (`self.Mesh`) (* (`KismetMathLibrary.GetForwardVector` (`self.K2_GetActorRotation`)) 10000.0) (`.BoneName` (`SkeletalMeshComponent.K2_GetClosestPointOnPhysicsAsset` _mesh ImpactoFinalLoc)) false)
  (`PrimitiveComponent.SetCollisionEnabled` (`self.CapsuleComponent`) "NoCollision")
  (`KismetSystemLibrary.K2_SetTimer` null "DestruirZombie" 5.0))

(event `DestruirZombie`
  (if (not (`self.EstaVivo?`))
    (`self.K2_DestroyActor`)))

(fn `UserConstructionScript`)
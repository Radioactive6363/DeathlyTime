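; GI_Gamemode, apparently a Game Instance, holds global music and a time value for the game.
; SpawnMusic plays SW_HunkTheme as a 2D sound that persists across level transitions without auto-destroying, keeping a reference so RestartMusic and StopMusic can control it.
; SaveTime stores a time value in GamemodeTime, and LoadTime writes it back through a by-ref parameter.
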(event `SpawnMusic`
  (bind _returnvalue (`GameplayStatics.SpawnSound2D` "/Game/Audios/AMBIENCE_SOUND/COMBAT/SW_HunkTheme.SW_HunkTheme" 1.0 1.0 0.0 null true false))
  (set `self.GlobalMusic` _returnvalue))

(event `RestartMusic`
  (`AudioComponent.Play` (`self.GlobalMusic`) 0.0))

(event `StopMusic`
  (`AudioComponent.Stop` (`self.GlobalMusic`)))

(fn `LoadTime`
  (params (TimeREF :type "Float (double-precision) (by ref)"))
  (`|VariableSetRef` TimeREF (`self.GamemodeTime`)))

(fn `SaveTime`
  (params (Time :type "Float (double-precision)"))
  (set `self.GamemodeTime` Time))
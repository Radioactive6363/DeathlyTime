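; BP_DoorMaster is a base door Blueprint for interactable doors that can optionally require a key.
; On BeginPlay it locks itself if a KeyRequired is set and binds to that key's pickup event to become openable.
; It answers interaction queries with an open or close prompt, its openable state and an interaction time.
; A completed interaction calls InteractionDoor, an empty event for child doors to override.
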(event `self.ReceiveBeginPlay`
  (bind _keyrequired (`self.KeyRequired`))
  (`/Engine/EditorBlueprintResources/StandardMacros.IsValid` _keyrequired
    (:`Is Valid`
      (set `self.CanBeOpened?` false)
      (set `self.NeedsKey?` true)
      (add `/Game/Blueprints/BP_DoorKey.OnPickedUpKey` _keyrequired (`|CreateDelegate` :!event `OpenDoorViaKey`)))
    (:`Is Not Valid`
      (set `self.CanBeOpened?` true))))

(event `OpenDoorViaKey`
  (set `self.CanBeOpened?` true)
  (set `self.NeedsKey?` false))

(event `/Game/Blueprints/Interfaces/BPI_InteractionInterface.DoInteractionResult`
  (params (HitResult :type "HitResult Structure") (Player :type "Actor Object Reference"))
  (`self.InteractionDoor`))

(event `InteractionDoor`)

(fn `CanBeInteracted`
  (returns (`Interactable?` :type Boolean))
  (return (`self.CanBeOpened?`)))

(fn `GetTime`
  (returns (Time :type "Float (double-precision)"))
  (return (`self._timeToInteract`)))

(fn `IsHoveringActor`
  (params (Hit :type "HitResult Structure") (Player :type "Actor Object Reference"))
  (returns (UpdatedText :type Text))
  (if (`self.IsOpen?`)
    (return "Close Door?")
    (else
      (return "Open Door?"))))

(fn `UserConstructionScript`
  (`parent.UserConstructionScript`))
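; Interactable sliding double door with a timed hold-E prompt, a key card message when it cannot be opened, and status lights.
; Timelines lerp the two panels in opposite directions, with separate events to open-and-lock, close-and-lock, lock or unlock.
; A dynamic light-function material and rect lights show state by color, and the construction script previews the starting state.
; Player overlap with the box toggles CanBeOpened while unlocked, disabling it inside.
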(event `self.InteractionDoor`
  (bind _door1baselocation (`self.Door1BaseLocation`))
  (bind _door2baselocation (`self.Door2BaseLocation`))
  (`self.DoorCheck`
    (:`OpenDoor`
      (`self.ChangeColor` (struct :`R` 0.065499 :`G` 1.0 :`A` 1.0))
      (bind (_direction _opendoorsalpha) (`Timeline|OpenDoors` :!label _label)
        (:`Update`
          (`self.SetLocationForObject` (`self.Door1`) _door1baselocation (+ _door1baselocation (`self.AmountToOpen`)) _opendoorsalpha)
          (`self.SetLocationForObject` (`self.Door2`) _door2baselocation (+ _door2baselocation (* (`self.AmountToOpen`) -1.0)) _opendoorsalpha))
        (:`Finished`
          (set `self.IsOpen?` (not (`self.IsOpen?`)))
          (set `self.IsOpening?` false))))
    (:`CloseDoor`
      (`self.ChangeColor` (struct :`R` 1.0 :`G` 0.917905 :`A` 1.0))
      (goto _label :!via `Reverse`))))

(event `Open and Lock`
  (bind _door1baselocation (`self.Door1BaseLocation`))
  (bind _door2baselocation (`self.Door2BaseLocation`))
  (`self.ChangeColor` (struct :`R` 1.0 :`A` 1.0))
  (bind (_direction _opendoorsalpha) (`Timeline|Timeline`)
    (:`Update`
      (`self.SetLocationForObject` (`self.Door1`) _door1baselocation (+ _door1baselocation (`self.AmountToOpen`)) _opendoorsalpha)
      (`self.SetLocationForObject` (`self.Door2`) _door2baselocation (+ _door2baselocation (* (`self.AmountToOpen`) -1.0)) _opendoorsalpha)
      (`self.LockUnlock` false))
    (:`Finished`
      (set `self.IsOpen?` (not (`self.IsOpen?`)))
      (set `self.IsOpening?` false))))

(event `Close and Lock`
  (bind _door2baselocation (`self.Door2BaseLocation`))
  (bind _door1baselocation (`self.Door1BaseLocation`))
  (`self.ChangeColor` (struct :`R` 1.0 :`A` 1.0))
  (bind (_direction _opendoorsalpha) (`Timeline|Timeline_0` :!via `Reverse`)
    (:`Update`
      (`self.SetLocationForObject` (`self.Door1`) _door1baselocation (+ _door1baselocation (`self.AmountToOpen`)) _opendoorsalpha)
      (`self.SetLocationForObject` (`self.Door2`) _door2baselocation (+ _door2baselocation (* (`self.AmountToOpen`) -1.0)) _opendoorsalpha)
      (`self.LockUnlock` false))
    (:`Finished`
      (set `self.IsOpen?` (not (`self.IsOpen?`)))
      (set `self.IsOpening?` false))))

(event `Lock`
  (`self.ChangeColor` (struct :`R` 1.0 :`A` 1.0))
  (`self.LockUnlock` false))

(event `Unlock`
  (`self.ChangeColor` (struct :`R` 1.0 :`G` 0.917905 :`A` 1.0))
  (`self.LockUnlock` true))

(event `self.Box.OnComponentBeginOverlap`
  (params (OverlappedComponent :type "PrimitiveComponent Object Reference") (OtherActor :type "Actor Object Reference") (OtherComp :type "PrimitiveComponent Object Reference") (OtherBodyIndex :type Integer) (bFromSweep :type Boolean) (SweepResult :type "HitResult Structure (by ref)"))
  (if (and (== OtherActor (`GameplayStatics.GetPlayerCharacter` 0)) (not (`self.IsLocked?`)))
    (set `self.CanBeOpened?` false)))

(event `self.Box.OnComponentEndOverlap`
  (params (OverlappedComponent :type "PrimitiveComponent Object Reference") (OtherActor :type "Actor Object Reference") (OtherComp :type "PrimitiveComponent Object Reference") (OtherBodyIndex :type Integer))
  (if (and (== OtherActor (`GameplayStatics.GetPlayerCharacter` 0)) (not (`self.IsLocked?`)))
    (set `self.CanBeOpened?` true)))

(fn `CanBeInteracted`
  (returns (`Interactable?` :type Boolean))
  (return (and (`self.CanBeOpened?`) (not (`self.IsOpening?`)))))

(fn `GetTime`
  (returns (Time :type "Float (double-precision)"))
  (return (`self._timeToInteract`)))

(fn `IsHoveringActor`
  (params (Hit :type "HitResult Structure") (Player :type "Actor Object Reference"))
  (returns (UpdatedText :type Text))
  (if (`self.CanBeOpened?`)
    (if (not (`self.IsOpening?`))
      (if (`self.IsOpen?`)
        (return "Close Door \nHold - E -")
        (else
          (return "Open Door  \nHold - E -")))
      (else
        (return "")))
    (else
      (return "Key card is required"))))

(fn `SetLocationForObject`
  (params (Target :type "SceneComponent Object Reference") (CurrentLocation :type "Vector Structure") (TargetLocation :type "Vector Structure") (Alpha :type "Float (single-precision)"))
  (`SceneComponent.K2_SetRelativeLocation` Target (`KismetMathLibrary.VLerp` CurrentLocation TargetLocation Alpha) false false))

(fn `UserConstructionScript`
  (`parent.UserConstructionScript`)
  (`|ExecutionSequence`
    (:`then_0`
      (bind _returnvalue (`KismetMaterialLibrary.CreateDynamicMaterialInstance` "/Game/Materials/M_LightFunction.M_LightFunction"))
      (bind _output_get (set `self.LightMaterials` _returnvalue))
      (`PrimitiveComponent.SetMaterial` (`self.LightMesh1`) 0 _output_get)
      (`PrimitiveComponent.SetMaterial` (`self.LightMesh2`) 0 _output_get)
      (`LightComponent.SetLightFunctionMaterial` (`self.RectLight1`) _returnvalue)
      (`LightComponent.SetLightFunctionMaterial` (`self.RectLight`) _returnvalue))
    (:`then_1`
      (`LocalLightComponent.SetAttenuationRadius` (`self.RectLight1`) (`self.LightAttenuation`))
      (`LocalLightComponent.SetAttenuationRadius` (`self.RectLight`) (`self.LightAttenuation`)))
    (:`then_2`
      (if (`self.IsOpen?`)
        (`self.ChangeColor` (struct :`R` 0.065499 :`G` 1.0 :`A` 1.0))
        (`SceneComponent.K2_SetRelativeLocation` (`self.Door1`) (+ (`self.Door1BaseLocation`) (`self.AmountToOpen`)) false false)
        (`SceneComponent.K2_SetRelativeLocation` (`self.Door2`) (+ (`self.Door2BaseLocation`) (* (`self.AmountToOpen`) -1.0)) false false)
        (else
          (if (`self.CanBeOpened?`)
            (`self.ChangeColor` (struct :`R` 1.0 :`G` 0.917905 :`A` 1.0))
            (else
              (`self.ChangeColor` (struct :`R` 1.0 :`G` 0.033789 :`A` 1.0))))
          (`SceneComponent.K2_SetRelativeLocation` (`self.Door1`) (`self.Door1BaseLocation`) false false)
          (`SceneComponent.K2_SetRelativeLocation` (`self.Door2`) (`self.Door2BaseLocation`) false false))))))
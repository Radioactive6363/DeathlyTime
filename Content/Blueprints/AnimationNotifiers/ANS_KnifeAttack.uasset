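; Animation notify state that applies knife damage during the player's attack animation.
; When the notify begins, it runs a single sphere trace between the root and end sockets of the current weapon of the owning BP_Player.
; If the hit actor implements BPI_Damage, it receives the weapon's damage through the IsDamagable message.
; The trace does not repeat over the rest of the notify window.
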(fn `Received_NotifyBegin`
  (params (MeshComp :type "SkeletalMeshComponent Object Reference") (Animation :type "AnimSequenceBase Object Reference") (TotalDuration :type "Float (single-precision)") (EventReference :type "AnimNotifyEventReference Structure (by ref)"))
  (returns (ReturnValue :type Boolean))
  (bind _asbp_player (cast `/Game/Blueprints/BP_Player` (`ActorComponent.GetOwner` MeshComp)))
  (bind _currentweapon (`/Game/Blueprints/BP_Player.CurrentWeapon` _asbp_player))
  (bind _outhit (`KismetSystemLibrary.SphereTraceSingle` MeshComp (`SceneComponent.GetSocketLocation` _currentweapon "b_knife_RootSocket") (`SceneComponent.GetSocketLocation` _currentweapon "b_knife_EndSocket") 100.0 "TraceTypeQuery3"))
  (bind (_bblockinghit _binitialoverlap _time _distance _location _impactpoint _normal _impactnormal _physmat _hitactor) (`GameplayStatics.BreakHitResult` _outhit))
  (if (`KismetSystemLibrary.DoesImplementInterface` _hitactor "/Game/Blueprints/Weapons/BPI_Damage.BPI_Damage_C")
    (message `/Game/Blueprints/Weapons/BPI_Damage.IsDamagable` _hitactor (`/Game/Blueprints/Weapons/BP_Weapon_Master.Damage` _currentweapon))))
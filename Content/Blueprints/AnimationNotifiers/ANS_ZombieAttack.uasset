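; ANS_ZombieAttack is an animation notify state that applies a melee hit for BP_DynamicEnemy during its attack animation.
; When the notify begins, a stationary sphere trace, with debug drawing enabled, checks a point just ahead of the enemy.
; If the hit actor implements BPI_Damage, it receives the enemy's damage amount and type through the interface.
; The check happens only once, at the start of the notify window.
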(fn `Received_NotifyBegin`
  (params (MeshComp :type "SkeletalMeshComponent Object Reference") (Animation :type "AnimSequenceBase Object Reference") (TotalDuration :type "Float (single-precision)") (EventReference :type "AnimNotifyEventReference Structure (by ref)"))
  (returns (ReturnValue :type Boolean))
  (bind _asbp_dynamic_enemy (cast `/Game/Blueprints/Enemies/DynamicEnemies/BP_DynamicEnemy` (`ActorComponent.GetOwner` MeshComp)))
  (bind _returnvalue (+ (`Actor.K2_GetActorLocation` _asbp_dynamic_enemy) (* (`Actor.GetActorForwardVector` _asbp_dynamic_enemy) 100.0)))
  (bind _outhit (`KismetSystemLibrary.SphereTraceSingle` :`WorldContextObject` MeshComp :`Start` _returnvalue :`End` _returnvalue :`Radius` 50.0 :`TraceChannel` "TraceTypeQuery5" :`DrawDebugType` "ForDuration"))
  (bind (_bblockinghit _binitialoverlap _time _distance _location _impactpoint _normal _impactnormal _physmat _hitactor) (`GameplayStatics.BreakHitResult` _outhit))
  (if (`KismetSystemLibrary.DoesImplementInterface` _hitactor "/Game/Blueprints/Weapons/BPI_Damage.BPI_Damage_C")
    (message `/Game/Blueprints/Weapons/BPI_Damage.IsDamagable` _hitactor (`/Game/Blueprints/Enemies/DynamicEnemies/BP_DynamicEnemy.Damage` _asbp_dynamic_enemy) (`/Game/Blueprints/Enemies/DynamicEnemies/BP_DynamicEnemy.TypeOfDamage` _asbp_dynamic_enemy))))
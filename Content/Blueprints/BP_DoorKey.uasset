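; Keycard pickup for doors that spins and bobs in place until the player interacts with it.
; A timeline drives mesh yaw and height, restarting itself on finish by calling RotateObject again.
; It answers interaction queries with a hover prompt, an interaction time and an always-interactable flag.
; On interaction it fires the OnPickedUpKey dispatcher and destroys itself.
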(event `self.ReceiveBeginPlay`
  (`parent.ReceiveBeginPlay`)
  (`self.RotateObject`))

(event `RotateObject`
  (bind _mesh (`self.Mesh`))
  (set `self.Relative Location` (`SceneComponent.RelativeLocation` (`self.Mesh`)))
  (bind (_direction _rotation _elevation) (`Timeline|Timeline` :!via `PlayFromStart`)
    (:`Update`
      (`SceneComponent.K2_SetRelativeRotation` _mesh (`KismetMathLibrary.MakeRotator` 0.0 0.0 _rotation) false false)
      (`SceneComponent.K2_SetRelativeLocation` _mesh (+ (`KismetMathLibrary.MakeVector` 0.0 0.0 _elevation) (`self.Relative Location`)) false false))
    (:`Finished`
      (`self.RotateObject`))))

(event `/Game/Blueprints/Interfaces/BPI_InteractionInterface.DoInteractionResult`
  (params (HitResult :type "HitResult Structure") (Player :type "Actor Object Reference"))
  (`self.OnPickedUpKey`)
  (`self.K2_DestroyActor`))

(fn `CanBeInteracted`
  (returns (`Interactable?` :type Boolean))
  (return true))

(fn `GetTime`
  (returns (Time :type "Float (double-precision)"))
  (return (`self._timeToInteract`)))

(fn `IsHoveringActor`
  (params (Hit :type "HitResult Structure") (Player :type "Actor Object Reference"))
  (returns (UpdatedText :type Text))
  (return "Pick KeyCard \nPress - E -"))

(fn `UserConstructionScript`
  (`parent.UserConstructionScript`))
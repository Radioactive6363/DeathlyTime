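; BP_Platform is a platform actor that shuttles back and forth between its current location and that location plus DesiredLocationAdd.
; The Movement event uses a FlipFlop to alternate playing and reversing a timeline at a rate set by SpeedPercentage, and re-triggers itself on finish to loop.
; Timeline updates lerp the position, teleporting without sweep.
; BeginPlay is empty, so nothing in this Blueprint starts the loop.
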(event `self.ReceiveBeginPlay`)

(event `Movement`
  (bind _templocation (`self.TempLocation`))
  (`TimelineComponent.SetPlayRate` (`self.MovementTimeline`) (/ (`self.SpeedPercentage`) 100.0))
  (`/Engine/EditorBlueprintResources/StandardMacros.FlipFlop`
    (:`A`
      (set `self.TempLocation` (`self.K2_GetActorLocation`))
      (bind (_direction _alpha) (`Timeline|MovementTimeline` :!via `PlayFromStart` :!label _label)
        (:`Update`
          (`self.K2_SetActorLocation` (`KismetMathLibrary.VLerp` _templocation (+ _templocation (`self.DesiredLocationAdd`)) _alpha) false true))
        (:`Finished`
          (`self.Movement`))))
    (:`B`
      (goto _label :!via `Reverse`))))

(fn `UserConstructionScript`)
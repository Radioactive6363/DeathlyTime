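; BP_MovableCar is an interactable car that reuses door logic to slide its mesh between a base position and an offset.
; A hold-E interaction passes through DoorCheck, then plays a sound and a delayed OpenDoors timeline that lerps relative location.
; A box overlap blocks interaction while the player is inside, with lock events and a key-card prompt alongside.
; The construction script places the mesh from its initial open state.
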(event `self.InteractionDoor`
  (bind _door1baselocation (`self.Door1BaseLocation`))
  (`self.DoorCheck`
    (:`OpenDoor`
      (set `self.IsOpen?` (not (`self.IsOpen?`)))
      (`GameplayStatics.PlaySoundAtLocation` "/Game/Audios/SFX/bbc_car---star_0009019.bbc_car---star_0009019" (`self.K2_GetActorLocation`) (struct) 1.0 1.0 0.0 null null null null)
      (`KismetSystemLibrary.Delay` 2.0)
      (bind (_direction _opendoorsalpha) (`Timeline|OpenDoors`)
        (:`Update`
          (`self.SetLocationForObject` (`self.SM_Car`) _door1baselocation (+ _door1baselocation (`self.AmountToOpen`)) _opendoorsalpha))
        (:`Finished`
          (set `self.IsOpening?` false))))))

(event `Open and Lock`
  (if (not (`self.IsOpen?`))
    (`TimelineComponent.Stop` (`self.OpenDoors`))
    (`self.LockUnlock` false
      (:`Result`
        (`Timeline|Timeline` :!label _label
          (:`Finished`
            (set `self.IsOpen?` (not (`self.IsOpen?`)))
            (set `self.IsOpening?` false)))))))

(event `Close and Lock`
  (if (`self.IsOpen?`)
    (`TimelineComponent.Stop` (`self.OpenDoors`))
    (`self.LockUnlock` false
      (:`Result`
        (goto _label :!via `Reverse`)))))

(event `Lock`
  (`self.LockUnlock` false))

(event `Unlock`
  (`self.LockUnlock` true))

(event `self.Box.OnComponentBeginOverlap`
  (params (OverlappedComponent :type "PrimitiveComponent Object Reference") (OtherActor :type "Actor Object Reference") (OtherComp :type "PrimitiveComponent Object Reference") (OtherBodyIndex :type Integer) (bFromSweep :type Boolean) (SweepResult :type "HitResult Structure (by ref)"))
  (if (and (== OtherActor (`GameplayStatics.GetPlayerCharacter` 0)) (not (`self.IsLocked?`)))
    (set `self.CanBeOpened?` false)))

(event `self.Box.OnComponentEndOverlap`
  (params (OverlappedComponent :type "PrimitiveComponent Object Reference") (OtherActor :type "Actor Object Reference") (OtherComp :type "PrimitiveComponent Object Reference") (OtherBodyIndex :type Integer))
  (if (and (== OtherActor (`GameplayStatics.GetPlayerCharacter` 0)) (not (`self.IsLocked?`)))
    (set `self.CanBeOpened?` true)))

(fn `CanBeInteracted`
  (returns (`Interactable?` :type Boolean))
  (return (and (`self.CanBeOpened?`) (not (`self.IsOpening?`)))))

(fn `GetTime`
  (returns (Time :type "Float (double-precision)"))
  (return (`self._timeToInteract`)))

(fn `IsHoveringActor`
  (params (Hit :type "HitResult Structure") (Player :type "Actor Object Reference"))
  (returns (UpdatedText :type Text))
  (if (not (`self.NeedsKey?`))
    (if (`self.CanBeOpened?`)
      (if (not (`self.IsOpening?`))
        (if (`self.IsOpen?`)
          (return "Close Door \nHold - E -")
          (else
            (return "Open Door  \nHold - E -"))))
      (else
        (return "")))
    (else
      (return "Key card is required"))))

(fn `SetLocationForObject`
  (params (Target :type "SceneComponent Object Reference") (CurrentLocation :type "Vector Structure") (TargetLocation :type "Vector Structure") (Alpha :type "Float (single-precision)"))
  (`SceneComponent.K2_SetRelativeLocation` Target (`KismetMathLibrary.VLerp` CurrentLocation TargetLocation Alpha) false false))

(fn `UserConstructionScript`
  (bind _sm_car (`self.SM_Car`))
  (`parent.UserConstructionScript`)
  (if (`self.IsOpen?`)
    (`SceneComponent.K2_SetRelativeLocation` _sm_car (+ (`self.Door1BaseLocation`) (`self.AmountToOpen`)) false false)
    (else
      (if (`self.CanBeOpened?`)
        _
        (else
          _))
      (`SceneComponent.K2_SetRelativeLocation` _sm_car (`self.Door1BaseLocation`) false false))))
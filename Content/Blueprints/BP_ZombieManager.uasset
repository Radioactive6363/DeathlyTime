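; BP_ZombieManager tracks spawned zombies and alerts them all when the player is detected.
; Spawn notifications add each zombie to the CurrentZombieCount array.
; On detection, it loops that array, casts each AI controller to IAC_Zombie, sets PlayerDetected and writes the player into the TargetPlayer Blackboard key, printing a debug message if the cast fails.
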(event `/Game/Blueprints/BPI_ZombieManagerComm.ZombiesSpawned`
  (params (ZombieReference :type "/Game/Zombie/BP_Zombie Object Reference"))
  (bind _returnvalue (`KismetArrayLibrary.Array_Add` (`self.CurrentZombieCount`) ZombieReference))
  (`KismetSystemLibrary.PrintString` (`KismetStringLibrary.Conv_IntToString` _returnvalue)))

(event `/Game/Blueprints/BPI_ZombieManagerComm.ZombieDetectedPlayer!`
  (params (PlayerReference :type "/Game/Blueprints/BP_Player Object Reference"))
  (for _array_element (`self.CurrentZombieCount`)
    (bind _asiac_zombie (cast `/Game/Zombie/IAC_Zombie` (`AIBlueprintHelperLibrary.GetAIController` _array_element))
      (:`then`
        (set `/Game/Zombie/IAC_Zombie.PlayerDetected?` true _asiac_zombie)
        (`BlackboardComponent.SetValueAsObject` (`AIController.Blackboard` _asiac_zombie) "TargetPlayer" PlayerReference))
      (:`CastFailed`
        (`KismetSystemLibrary.PrintString` "Falla Deteccion Jugador en Manager")))))

(fn `UserConstructionScript`)
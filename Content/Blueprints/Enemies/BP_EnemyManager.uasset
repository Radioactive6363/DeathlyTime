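; Enemy manager that tracks live enemies in an array and spreads player detection across the group.
; Events register spawned enemies and remove valid ones on request, while CheckLimitOfEnemies reports whether the count equals MaxZombieCount.
; On detection, it loops through every tracked enemy, casts its AI controller to IAC_DynamicEnemy and passes the player to DetectedPlayer.
; CheckLength prints the count for debugging, and MakeArray is empty.
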(event `/Game/Blueprints/Enemies/BPI_ZombieManagerComm.EnemySpawned`
  (params (EnemyReference :type "/Game/Blueprints/Enemies/BP_EnemyBase Object Reference"))
  (`KismetArrayLibrary.Array_Add` (`self.CurrentEnemyCount`) EnemyReference))

(event `/Game/Blueprints/Enemies/BPI_ZombieManagerComm.EnemyDetectedPlayer!`
  (params (PlayerReference :type "/Game/Blueprints/BP_Player Object Reference"))
  (for _array_element (`self.CurrentEnemyCount`)
    (bind _asiac_dynamic_enemy (cast `/Game/Blueprints/Enemies/IAC_DynamicEnemy` (`AIBlueprintHelperLibrary.GetAIController` _array_element)))
    (`/Game/Blueprints/Enemies/IAC_DynamicEnemy.DetectedPlayer` _asiac_dynamic_enemy PlayerReference)))

(event `/Game/Blueprints/Enemies/BPI_ZombieManagerComm.DeleteEnemiesFromArray`
  (params (EnemyToDelete :type "/Game/Blueprints/Enemies/BP_EnemyBase Object Reference"))
  (`/Engine/EditorBlueprintResources/StandardMacros.IsValid` EnemyToDelete
    (:`Is Valid`
      (`KismetArrayLibrary.Array_RemoveItem` (`self.CurrentEnemyCount`) EnemyToDelete))))

(event `/Game/Blueprints/Enemies/BPI_ZombieManagerComm.CheckLength`
  (`KismetSystemLibrary.PrintString` (`KismetStringLibrary.Conv_IntToString` (`KismetArrayLibrary.Array_Length` (`self.CurrentEnemyCount`)))))

(fn `CheckLimitOfEnemies`
  (returns (`isAtLimit?` :type Boolean))
  (return (== (`KismetArrayLibrary.Array_Length` (`self.CurrentEnemyCount`)) (`self.MaxZombieCount`))))

(fn `MakeArray`
  (locals (Array :type "Array of /Game/Blueprints/Enemies/BP_EnemyBase Object Reference")))

(fn `UserConstructionScript`)
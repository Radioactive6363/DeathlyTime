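; Zombie enemy Blueprint that handles running speed, death and removal from play.
; SetSpeed applies the running max walk speed to character movement.
; On death it detaches its controller, plays a death animation, disables capsule collision, switches to ragdoll physics after a short delay and starts a timer.
; DestroyZombie tells BP_EnemyManager to drop it from the enemy array, then destroys the actor.
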(event `self.ReceiveBeginPlay`
  (`parent.ReceiveBeginPlay`))

(event `SetSpeed`
  (set `CharacterMovementComponent.MaxWalkSpeed` (`self.RunningMaxSpeed`) (`self.CharacterMovement`)))

(event `self.OnDeathEvents`
  (`self.DetachFromControllerPendingDestroy`)
  (`SkeletalMeshComponent.PlayAnimation` (`self.Mesh`) (`self.DeathAnimationToPlay`) false)
  (`PrimitiveComponent.SetCollisionEnabled` (`self.CapsuleComponent`) "NoCollision")
  (`KismetSystemLibrary.Delay` 0.5)
  (`PrimitiveComponent.SetSimulatePhysics` (`self.Mesh`) true)
  (`KismetSystemLibrary.K2_SetTimerDelegate` (`|CreateDelegate` :!event `DestroyZombie`) 5.0))

(event `DestroyZombie`
  (bind _returnvalue (`GameplayStatics.GetActorOfClass` "/Game/Blueprints/Enemies/BP_EnemyManager.BP_EnemyManager_C"))
  (message `/Game/Blueprints/Enemies/BPI_ZombieManagerComm.DeleteEnemiesFromArray` _returnvalue self)
  (`self.K2_DestroyActor`))

(fn `UserConstructionScript`
  (`parent.UserConstructionScript`))
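; BP_DynamicEnemy is a base Blueprint for dynamic enemies, handling life, damage and death.
; Life starts at MaxLife, and the IsDamagable event passes damage to ACLifeController, then triggers Death when life reaches zero or below.
; Death is guarded by an Alive flag so it fires OnDeathEvents only once.
; OnDeathEvents is an empty override hook, and AttackPlayer is a stub returning zero.
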(event `self.ReceiveBeginPlay`
  (set `self.CurrentLife` (`self.MaxLife`)))

(event `/Game/Blueprints/Weapons/BPI_Damage.IsDamagable`
  (params (Damage :type "Float (double-precision)") (TimeDamage :type "Float (double-precision)"))
  (`|ExecutionSequence`
    (:`then_0`
      (`/Game/Blueprints/ActorComponents/AC_LifeController.ChangeHealthDirect` (`self.AC_LifeController`) (`self.CurrentLife`) Damage))
    (:`then_1`
      (if (<= (`self.CurrentLife`) 0.0)
        (`self.Death`)))))

(event `Death`
  ; On Death
  (if (`self.Alive?`)
    (set `self.Alive?` false)
    (`self.OnDeathEvents`)))

(event `OnDeathEvents`)

(fn `AttackPlayer`
  (returns (MontageDuration :type "Float (double-precision)"))
  (return 0.0))

(fn `UserConstructionScript`)
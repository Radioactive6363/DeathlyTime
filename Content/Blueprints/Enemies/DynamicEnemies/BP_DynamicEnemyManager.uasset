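; Manager that keeps a registry of live dynamic zombie enemies and can check whether their count equals the maximum.
; Spawned enemies join the array, and each removal also reloads the player's main rifle, obtained at BeginPlay through BP_Player.
; A detection event alerts the registered zombies through their AI controllers, stopping at a failed cast.
; It can also kill all tracked zombies or print the count.
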(event `self.ReceiveBeginPlay`
  (bind _returnvalue (`GameplayStatics.GetActorOfClass` "/Game/Blueprints/BP_Player.BP_Player_C"))
  (`/Engine/EditorBlueprintResources/StandardMacros.IsValid` _returnvalue
    (:`Is Valid`
      (add `/Game/Blueprints/BP_Player.UpdMainWeapon` _returnvalue (delegate `WeaponToReload`)))))

(event `WeaponToReload`
  (params (Rifle :type "/Game/Blueprints/Weapons/BP_Weapon_Rifle Object Reference"))
  (set `self.MainRifleWeapon` Rifle))

(event `/Game/Blueprints/Enemies/DynamicEnemies/BPI_DynamicEnemyMan.EnemySpawned`
  (params (EnemyReference :type "/Game/Blueprints/Enemies/DynamicEnemies/BP_DynamicEnemy Object Reference"))
  (`KismetArrayLibrary.Array_Add` (`self.CurrentEnemyCount`) EnemyReference))

(event `/Game/Blueprints/Enemies/DynamicEnemies/BPI_DynamicEnemyMan.EnemyDetectedPlayer!`
  (for _array_element (`self.CurrentEnemyCount`)
    (bind _asiac_zombie_enemy (cast `/Game/Blueprints/Enemies/DynamicEnemies/IAC_ZombieEnemy` (`AIBlueprintHelperLibrary.GetAIController` _array_element)))
    (`/Game/Blueprints/Enemies/IAC_MasterEnemy.OnDetectedPlayer` _asiac_zombie_enemy)))

(event `/Game/Blueprints/Enemies/DynamicEnemies/BPI_DynamicEnemyMan.DeleteEnemiesFromArray`
  (params (EnemyToDelete :type "/Game/Blueprints/Enemies/DynamicEnemies/BP_DynamicEnemy Object Reference"))
  (`/Engine/EditorBlueprintResources/StandardMacros.IsValid` EnemyToDelete
    (:`Is Valid`
      (`KismetArrayLibrary.Array_RemoveItem` (`self.CurrentEnemyCount`) EnemyToDelete)
      (`/Game/Blueprints/Weapons/BP_Weapon_Rifle.ReloadWeapon` (`self.MainRifleWeapon`)))))

(event `/Game/Blueprints/Enemies/DynamicEnemies/BPI_DynamicEnemyMan.RemoveAllZombies`
  (for _array_element (`self.CurrentEnemyCount`)
    (`/Engine/EditorBlueprintResources/StandardMacros.IsValid` _array_element
      (:`Is Valid`
        (`/Game/Blueprints/Enemies/DynamicEnemies/BP_DynamicEnemy.Death` _array_element)))))

(event `/Game/Blueprints/Enemies/DynamicEnemies/BPI_DynamicEnemyMan.CheckLength`
  (`KismetSystemLibrary.PrintString` (`KismetStringLibrary.Conv_IntToString` (`KismetArrayLibrary.Array_Length` (`self.CurrentEnemyCount`)))))

(fn `CheckLimitOfEnemies`
  (returns (`isAtLimit?` :type Boolean))
  (return (== (`KismetArrayLibrary.Array_Length` (`self.CurrentEnemyCount`)) (`self.MaxZombieCount`))))

(fn `MakeArray`
  (locals (Array :type "Array of /Game/Blueprints/Enemies/DynamicEnemies/BP_DynamicEnemy Object Reference")))

(fn `UserConstructionScript`)
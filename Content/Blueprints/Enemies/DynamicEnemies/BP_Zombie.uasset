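; BP_Zombie is a dynamic enemy zombie that attacks with a random montage and picks a random skeletal mesh at construction.
; It caches the BP_DynamicEnemyManager on BeginPlay.
; On death it detaches its controller, plays a death animation, disables capsule collision and has the manager remove it from its array.
; It switches to ragdoll physics after a short delay, then starts a timer, apparently for DestroyZombie cleanup.
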(event `self.ReceiveBeginPlay`
  (`parent.ReceiveBeginPlay`)
  (bind _returnvalue (`GameplayStatics.GetActorOfClass` "/Game/Blueprints/Enemies/DynamicEnemies/BP_DynamicEnemyManager.BP_DynamicEnemyManager_C"))
  (set `self.Manager` _returnvalue))

(event `self.OnDeathEvents`
  (`self.DetachFromControllerPendingDestroy`)
  (`SkeletalMeshComponent.PlayAnimation` (`self.Mesh`) (`self.DeathAnimationToPlay`) false)
  (`PrimitiveComponent.SetCollisionEnabled` (`self.CapsuleComponent`) "NoCollision")
  (message `/Game/Blueprints/Enemies/DynamicEnemies/BPI_DynamicEnemyMan.DeleteEnemiesFromArray` (`self.Manager`) self)
  (`KismetSystemLibrary.Delay` 0.5)
  (`PrimitiveComponent.SetSimulatePhysics` (`self.Mesh`) true)
  (`KismetSystemLibrary.K2_SetTimerDelegate` (`|CreateDelegate` :!event `DestroyZombie`) 5.0))

(event `DestroyZombie`
  (`self.K2_DestroyActor`))

(fn `AttackPlayer`
  (returns (MontageDuration :type "Float (double-precision)"))
  (bind _returnvalue (`self.PlayAnimMontage` (`KismetArrayLibrary.Array_Random` (`self.Montage to Play`))))
  (return _returnvalue))

(fn `UserConstructionScript`
  (bind _meshes (`self.Meshes`))
  (`parent.UserConstructionScript`)
  (`SkeletalMeshComponent.SetSkeletalMeshAsset` (`self.Mesh`) (`|GetArrayItem` _meshes (`KismetMathLibrary.RandomInteger` (- (`KismetArrayLibrary.Array_Length` _meshes) 1)))))
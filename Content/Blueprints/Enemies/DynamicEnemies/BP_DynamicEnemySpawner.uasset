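; Enemy spawner that creates actors of a configurable class at random reachable points within a radius, previewed by a construction-script debug sphere.
; SpawnerType selects looping-timer spawning (counted, unlimited or time-spread) or instant batches; finite modes then destroy the spawner.
; Each spawn first checks BP_DynamicEnemyManager's enemy limit and reports back to it.
; Depending on mode, the zombie AI controller gets blackboard spawn values, immediate player detection or both.
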(event `self.ReceiveBeginPlay`
  (if (`self.AllowedInstantSpawning?`)
    (`KismetSystemLibrary.Delay` 0.2)
    (`self.StartSpawner`)))

(event `StartSpawnerWithTimer`
  (params (TimeDelay :type "Float (double-precision)"))
  (if (not (<= TimeDelay 0.0))
    (`KismetSystemLibrary.K2_SetTimerDelegate` (`|CreateDelegate` :!event `StartSpawner`) TimeDelay)))

(event `ContinuousWLimit`
  ; Spawns Enemy Continuosly with Limit
  (if (<= (`self.TempSpawner`) (`self.AmountDesired`))
    (`/Engine/EditorBlueprintResources/StandardMacros.IncrementInt` (`self.TempSpawner`)
      (:`  `
        (bind _enemyspawned (`self.SpawnActor`))
        (`self.SetSpawnValuesToEnemy` _enemyspawned)
        (`self.SetPlayerDetected` _enemyspawned)))
    (else
      (`KismetSystemLibrary.K2_ClearAndInvalidateTimerHandle` (`self.WithLimit`))
      (`self.DestroySpawner`))))

(event `StartSpawner`
  (`KismetSystemLibrary.Delay` 0.2)
  (switch `/Game/Blueprints/Enemies/DynamicEnemies/Enum_TypeOfSpawner` (`self.SpawnerType`)
    (:`NewEnumerator8`
      ; Spawns Enemy Continuosly with Limit
      (bind _returnvalue (`KismetSystemLibrary.K2_SetTimerDelegate` (delegate `ContinuousWLimit`) (`self.TimeToSpawn`) true))
      (set `self.WithLimit` _returnvalue))
    (:`NewEnumerator0`
      ; Spawns Enemy Continuosly but with NO limit
      (bind _returnvalue_2 (`KismetSystemLibrary.K2_SetTimerDelegate` (delegate `ContinuousNLimit`) (`self.TimeToSpawn`) true))
      (set `self.NoLimit` _returnvalue_2))
    (:`NewEnumerator10`
      ; Spawns Enemy Continuosly But binded by time
      (bind _returnvalue_3 (`KismetSystemLibrary.K2_SetTimerDelegate` (delegate `ContinuousTimeBinded`) (/ (`self.TimeToSpawn`) (`self.AmountDesired`)) true))
      (set `self.WithLimit` _returnvalue_3))
    (:`NewEnumerator7`
      ; Spawns Enemy on an Instant Way
      (for _ (range (`self.AmountDesired`))
        (bind _enemyspawned (`self.SpawnActor`))
        (`self.SetSpawnValuesToEnemy` _enemyspawned))
      (`self.DestroySpawner`))
    (:`NewEnumerator9`
      ; Spawns Enemy on an Instant Way + AlreadyDetected
      (for _ (range (`self.AmountDesired`))
        (bind _enemyspawned_2 (`self.SpawnActor`))
        (`self.SetPlayerDetected` _enemyspawned_2))
      (`self.DestroySpawner`))))

(event `ContinuousNLimit`
  ; Spawns Enemy Continuosly but with NO limit
  (bind _enemyspawned (`self.SpawnActor`))
  (`self.SetPlayerDetected` _enemyspawned))

(event `ContinuousTimeBinded`
  ; Spawns Enemy Continuosly But binded by time
  (if (<= (`self.TempSpawner`) (`self.AmountDesired`))
    (`/Engine/EditorBlueprintResources/StandardMacros.IncrementInt` (`self.TempSpawner`)
      (:`  `
        (bind _enemyspawned (`self.SpawnActor`))
        (`self.SetSpawnValuesToEnemy` _enemyspawned)
        (`self.SetPlayerDetected` _enemyspawned)))
    (else
      (`KismetSystemLibrary.K2_ClearAndInvalidateTimerHandle` (`self.WithLimit`))
      (`self.DestroySpawner`))))

(event `SetSpawnValuesToEnemy`
  (params (ControlledActor :type "Actor Object Reference"))
  ; Set Values On BlackBoard on one zombie
  (bind _asiac_zombie_enemy (cast `/Game/Blueprints/Enemies/DynamicEnemies/IAC_ZombieEnemy` (`AIBlueprintHelperLibrary.GetAIController` ControlledActor)))
  (`/Game/Blueprints/Enemies/DynamicEnemies/IAC_ZombieEnemy.InitializeBlackboard` _asiac_zombie_enemy (`self.K2_GetActorLocation`) (`self.SpawnRadius`)))

(event `DestroySpawner`
  (`KismetSystemLibrary.Delay` 3.0)
  (`self.K2_DestroyActor`))

(event `SetPlayerDetected`
  (params (ControlledActor :type "Actor Object Reference"))
  (bind _asiac_zombie_enemy (cast `/Game/Blueprints/Enemies/DynamicEnemies/IAC_ZombieEnemy` (`AIBlueprintHelperLibrary.GetAIController` ControlledActor)))
  (`/Game/Blueprints/Enemies/IAC_MasterEnemy.OnDetectedPlayer` _asiac_zombie_enemy))

(event `StopSpawner`
  (`KismetSystemLibrary.K2_ClearAndInvalidateTimerHandle` (`self.WithLimit`))
  (`KismetSystemLibrary.K2_ClearAndInvalidateTimerHandle` (`self.NoLimit`)))

(fn `SpawnActor`
  (returns (EnemySpawned :type "/Game/Blueprints/Enemies/DynamicEnemies/BP_DynamicEnemy Object Reference"))
  (bind _returnvalue (`GameplayStatics.GetActorOfClass` "/Game/Blueprints/Enemies/DynamicEnemies/BP_DynamicEnemyManager.BP_DynamicEnemyManager_C"))
  (bind _isatlimit_ (message `/Game/Blueprints/Enemies/DynamicEnemies/BPI_DynamicEnemyMan.CheckLimitOfEnemies` _returnvalue))
  (if (not _isatlimit_)
    (bind _returnvalue_2 (`self.SpawnLocation`))
    (message `/Game/Blueprints/Enemies/DynamicEnemies/BPI_DynamicEnemyMan.EnemySpawned` _returnvalue _returnvalue_2)
    (return _returnvalue_2)))

(fn `SpawnLocation`
  (returns (ReturnValue :type "/Game/Blueprints/Enemies/DynamicEnemies/BP_DynamicEnemy Object Reference"))
  (bind (_returnvalue_roll _returnvalue_pitch _returnvalue_yaw) (`KismetMathLibrary.BreakRotator` (`KismetMathLibrary.RandomRotator` true)))
  (bind _randomlocation (`NavigationSystemV1.K2_GetRandomReachablePointInRadius` (`self.K2_GetActorLocation`) (`self.SpawnRadius`) null null))
  (bind _returnvalue (`|SpawnActorFromClass` (`self.EnemyToSpawn`) (`KismetMathLibrary.MakeTransform` (`KismetMathLibrary.MakeVector` (.x _randomlocation) (.y _randomlocation)) (`KismetMathLibrary.MakeRotator` 0.0 0.0 _returnvalue_yaw)) "AdjustIfPossibleButAlwaysSpawn" "MultiplyWithRoot" null (`self.CustomDamage`) null))
  (return _returnvalue))

(fn `UserConstructionScript`
  (`KismetSystemLibrary.DrawDebugSphere` (`self.K2_GetActorLocation`) (`self.SpawnRadius`) 12 (struct :`G` 0.37778 :`B` 1.0 :`A` 0.25) 1.0))
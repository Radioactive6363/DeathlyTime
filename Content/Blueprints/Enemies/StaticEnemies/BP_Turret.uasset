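; Static enemy turret that idly sweeps its head to random yaws, then tracks and shoots the player inside its detection sphere.
; A timeline and delay timer drive the search, while looping timers handle interpolated tracking and firing, with a warning sound on detection.
; Shots are line traces that send damage through BPI_Damage and spawn explosion effects.
; Leaving the sphere, whose radius is set at construction, unbinds the warning callback and resumes searching.
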(event `self.ReceiveBeginPlay`
  (`self.ChangeRotation`))

(event `ChangeRotation`
  ; Searching State
  (set `self.TempRotation` (`SceneComponent.RelativeRotation` (`self.Head`)))
  (`TimelineComponent.SetPlayRate` (`self.RotationTime`) (`KismetMathLibrary.RandomFloatInRange` 0.5 2.0))
  (set `self.Temp Z Rotation` (`KismetMathLibrary.RandomFloatInRange` -90.0 90.0))
  (bind (_direction _alpharotation) (`Timeline|RotationTime` :!via `PlayFromStart` :!label _label)
    (:`Update`
      (`SceneComponent.K2_SetRelativeRotation` (`self.Head`) (`KismetMathLibrary.RLerp` (`self.TempRotation`) (`KismetMathLibrary.MakeRotator` 0.0 0.0 (`self.Temp Z Rotation`)) _alpharotation) false false))
    (:`Finished`
      (bind _returnvalue (`KismetSystemLibrary.K2_SetTimerDelegate` (`|CreateDelegate` :!event `ChangeRotation`) 2.0 false true))
      (set `self.RotationTimer` _returnvalue))))

(event `StopRotationTimeline`
  ; Searching State
  (`KismetSystemLibrary.K2_ClearAndInvalidateTimerHandle` (`self.RotationTimer`))
  (goto _label :!via `Stop`))

(event `self.SphereCollision.OnComponentBeginOverlap`
  (params (OverlappedComponent :type "PrimitiveComponent Object Reference") (OtherActor :type "Actor Object Reference") (OtherComp :type "PrimitiveComponent Object Reference") (OtherBodyIndex :type Integer) (bFromSweep :type Boolean) (SweepResult :type "HitResult Structure (by ref)"))
  ; Found Target State
  (if (== OtherActor (`GameplayStatics.GetPlayerCharacter` 0))
    (`self.StopRotationTimeline`)
    (set `self.Target` OtherActor)
    (`|ExecutionSequence`
      (:`then_0`
        (bind _returnvalue (`KismetSystemLibrary.K2_SetTimerDelegate` (`|CreateDelegate` :!event `RotateTowardsTarget`) 0.01 true true))
        (set `self.TrackingTimer` _returnvalue))
      (:`then_1`
        (bind _returnvalue_2 (`GameplayStatics.SpawnSoundAtLocation` "/Game/Audios/SW_WarningSoundTurret.SW_WarningSoundTurret" (`self.K2_GetActorLocation`) (struct) 1.0 1.0 0.0 null null))
        (bind _output_get (set `self.WarningSound` _returnvalue_2))
        (add `AudioComponent.OnAudioFinished` _output_get (`|CreateDelegate` :!event `StartFiringTimer`))))))

(event `StartFiringTimer`
  ; Found Target State
  (bind _returnvalue (`KismetSystemLibrary.K2_SetTimerDelegate` (`|CreateDelegate` :!event `Fire`) (`self.FireRate`) true true))
  (set `self.FireRateTimer` _returnvalue))

(event `Fire`
  ; Found Target State
  ;; Shoot Target
  (`self.PlayFireEffects`)
  (bind _output_get (`/Game/Blueprints/FunctionUtilities/BP_TraceUtilities.LineTrace` (`self.Head`) (* (`self.FireDistance`) -1.0) "TraceTypeQuery5" "ForDuration"))
  (`|ExecutionSequence`
    (:`then_0`
      (bind (_bblockinghit _binitialoverlap _time _distance _location _impactpoint _normal _impactnormal _physmat _hitactor) (`GameplayStatics.BreakHitResult` _output_get))
      (if (`KismetSystemLibrary.DoesImplementInterface` _hitactor "/Game/Blueprints/Weapons/BPI_Damage.BPI_Damage_C")
        (message `/Game/Blueprints/Weapons/BPI_Damage.IsDamagable` _hitactor (`self.Damage`) (`self.TypeOfDamage`))))
    (:`then_1`
      (`GameplayStatics.SpawnEmitterAtLocation` "/Game/ExtraContent/StarterContent/Particles/P_Explosion.P_Explosion" _location))))

(event `PlayFireEffects`
  ; Found Target State
  ;; Shoot Target
  (`GameplayStatics.SpawnSoundAttached` "/Game/ExtraContent/FPWeapon/Audio/FirstPersonTemplateWeaponFire02.FirstPersonTemplateWeaponFire02" (`self.Head`) "Muzzle" (0.0 0.0 0.0) (struct) "KeepRelativeOffset" false 1.0 1.0 0.0 null null)
  (`GameplayStatics.SpawnEmitterAttached` "/Game/ExtraContent/StarterContent/Particles/P_Explosion.P_Explosion" (`self.Head`) "Muzzle" (0.0 0.0 0.0) (struct) (5.0 5.0 5.0) "KeepRelativeOffset" true "AutoRelease"))

(event `RotateTowardsTarget`
  (bind _target (`self.Target`))
  ; Found Target State
  ;; Rotate Towards Target
  (`/Engine/EditorBlueprintResources/StandardMacros.IsValid` _target
    (:`Is Valid`
      (`SceneComponent.K2_SetWorldRotation` (`self.Head`) (`KismetMathLibrary.RInterpTo` (`SceneComponent.K2_GetComponentRotation` (`self.Head`)) (`KismetMathLibrary.FindLookAtRotation` (`self.K2_GetActorLocation` _target) (`self.K2_GetActorLocation`)) (`GameplayStatics.GetWorldDeltaSeconds`) (`self.RotationSpeed`)) false false))))

(event `self.SphereCollision.OnComponentEndOverlap`
  (params (OverlappedComponent :type "PrimitiveComponent Object Reference") (OtherActor :type "Actor Object Reference") (OtherComp :type "PrimitiveComponent Object Reference") (OtherBodyIndex :type Integer))
  (bind _warningsound (`self.WarningSound`))
  ; Return to Searching State
  (if (== OtherActor (`GameplayStatics.GetPlayerCharacter` 0))
    (`self.RestartTurret`)
    (`/Engine/EditorBlueprintResources/StandardMacros.IsValid` _warningsound
      (:`Is Valid`
        (clear `AudioComponent.OnAudioFinished` _warningsound)))))

(event `RestartTurret`
  ; Return to Searching State
  (`KismetSystemLibrary.K2_ClearAndInvalidateTimerHandle` (`self.TrackingTimer`))
  (`KismetSystemLibrary.K2_ClearAndInvalidateTimerHandle` (`self.FireRateTimer`))
  (set `self.Target` null)
  (`self.ChangeRotation`))

(fn `UserConstructionScript`
  (`parent.UserConstructionScript`)
  (`SphereComponent.SetSphereRadius` (`self.SphereCollision`) (`self.DetectionZoneRadius`) true))
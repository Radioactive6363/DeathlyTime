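; AI controller for dynamic enemies that runs the BT_Zombie behavior tree on BeginPlay.
; InitializeBlackboard writes the spawn location and radius to the blackboard.
; Until the player is detected, successful sight or hearing of the player character is reported to BP_EnemyManager.
; A separate DetectedPlayer event sets the detection flag and stores the player as the blackboard's TargetPlayer.
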(event `self.ReceiveBeginPlay`
  (`self.RunBehaviorTree` "/Game/Blueprints/Enemies/BT_Zombie.BT_Zombie"))

(event `InitializeBlackboard`
  (params (SpawnLocation :type "Vector Structure") (SpawnRadius :type "Float (double-precision)"))
  (bind _blackboard (`self.Blackboard`))
  (`|ExecutionSequence`
    (:`then_0`
      (`BlackboardComponent.SetValueAsVector` _blackboard "SpawnLocation" SpawnLocation))
    (:`then_1`
      (`BlackboardComponent.SetValueAsFloat` _blackboard "SpawnRadius" SpawnRadius))))

(event `self.AIPerception.OnTargetPerceptionUpdated`
  (params (Actor :type "Actor Object Reference") (Stimulus :type "AIStimulus Structure"))
  (bind _returnvalue (`AIPerceptionSystem.GetSenseClassForStimulus` Stimulus))
  (if (and (or (== _returnvalue "/Script/AIModule.AISense_Sight") (== _returnvalue "/Script/AIModule.AISense_Hearing")) (== (`GameplayStatics.GetPlayerCharacter` 0) Actor) (not (`self.PlayerDetected?`)))
    (if (`.bSuccessfullySensed` (break `AIStimulus` Stimulus))
      (bind _returnvalue_2 (`GameplayStatics.GetActorOfClass` "/Game/Blueprints/Enemies/BP_EnemyManager.BP_EnemyManager_C"))
      (bind _asbp_player (cast `/Game/Blueprints/BP_Player` Actor))
      (message `/Game/Blueprints/Enemies/BPI_ZombieManagerComm.EnemyDetectedPlayer!` _returnvalue_2 _asbp_player))))

(event `DetectedPlayer`
  (params (PlayerReference :type "Object Object Reference"))
  (set `self.PlayerDetected?` true)
  (`BlackboardComponent.SetValueAsObject` (`self.Blackboard`) "TargetPlayer" PlayerReference))

(fn `UserConstructionScript`)
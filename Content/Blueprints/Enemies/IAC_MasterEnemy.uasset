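; Base AI controller for enemies that runs a behavior tree and handles detection of the player through sight and hearing.
; A successfully sensed stimulus from the player fires the overridable OnPerceptionDetectedPlayer hook, empty here, as long as the player is not yet detected.
; A separate overridable OnDetectedPlayer event, not called in this graph, sets the detected flag and writes the player to the TargetPlayer blackboard key.
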(event `self.ReceiveBeginPlay`
  (`self.RunBehaviorTree` (`self.BTAsset`)))

(event `self.AIPerception.OnTargetPerceptionUpdated`
  (params (Actor :type "Actor Object Reference") (Stimulus :type "AIStimulus Structure"))
  (bind _returnvalue (`AIPerceptionSystem.GetSenseClassForStimulus` Stimulus))
  (if (and (or (== _returnvalue "/Script/AIModule.AISense_Sight") (== _returnvalue "/Script/AIModule.AISense_Hearing")) (== (`GameplayStatics.GetPlayerCharacter` 0) Actor) (not (`self.PlayerDetected?`)))
    (if (`.bSuccessfullySensed` (break `AIStimulus` Stimulus))
      (`self.OnPerceptionDetectedPlayer`))))

(event `OnPerceptionDetectedPlayer`)

(event `OnDetectedPlayer`
  (set `self.PlayerDetected?` true)
  (`BlackboardComponent.SetValueAsObject` (`self.Blackboard`) "TargetPlayer" (`GameplayStatics.GetPlayerCharacter` 0)))

(fn `UserConstructionScript`)
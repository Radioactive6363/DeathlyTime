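; BP_AnimationUtilities is an animation utility Blueprint with one helper, GetSectionEndTime, for finding the time at which a montage section ends.
; It jumps the montage to the section's end on the given AnimInstance, then returns the resulting montage position.
; The lookup moves the montage's playback position and does not restore it, so it is not a side-effect-free query.
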(fn `GetSectionEndTime`
  (params (AnimMontage :type "AnimMontage Object Reference") (AnimInstance :type "AnimInstance Object Reference") (Section :type Name))
  (returns (EndTimeSection :type "Float (double-precision)"))
  (locals (Montage :type "AnimMontage Object Reference") (`Anim Instance` :type "AnimInstance Object Reference") (MontageSection :type Name))
  (set `local.Montage` AnimMontage)
  (set `local.Anim Instance` AnimInstance)
  (set `local.MontageSection` Section)
  (`AnimInstance.Montage_JumpToSectionsEnd` (`local.Anim Instance`) (`local.MontageSection`) (`local.Montage`))
  (return (`AnimInstance.Montage_GetPosition` (`local.Anim Instance`) (`local.Montage`))))
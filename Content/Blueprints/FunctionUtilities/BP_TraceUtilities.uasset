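; Utility Blueprint of forward trace helpers, with hover-target tracking for hit results.
; Line, sphere and multi-sphere traces run from just ahead of a given component along its forward vector, with configurable length and debug drawing.
; The multi-sphere trace uses a fixed channel, while the others take one as input.
; CheckActor stores the hit actor and component as hovered, but clears both when the same pair is passed again.
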(fn `CheckActor`
  (params (HitResult :type "HitResult Structure (by ref)"))
  (returns (HoveredComponent :type "PrimitiveComponent Object Reference") (HoveredTarget :type "Actor Object Reference"))
  (locals (_currentHoveredTarget :type "Actor Object Reference") (_currentHoveredComponent :type "PrimitiveComponent Object Reference"))
  (bind (_bblockinghit _binitialoverlap _time _distance _location _impactpoint _normal _impactnormal _physmat _hitactor _hitcomponent) (`GameplayStatics.BreakHitResult` HitResult))
  (bind (_bblockinghit_2 _binitialoverlap_2 _time_2 _distance_2 _location_2 _impactpoint_2 _normal_2 _impactnormal_2 _physmat_2 _hitactor_2 _hitcomponent_2) (`GameplayStatics.BreakHitResult` HitResult))
  (if (and (== _hitactor_2 (`local._currentHoveredTarget`)) (== _hitcomponent_2 (`local._currentHoveredComponent`)))
    (set `local._currentHoveredTarget` null)
    (set `local._currentHoveredComponent` null)
    (else
      (set `local._currentHoveredTarget` _hitactor)
      (set `local._currentHoveredComponent` _hitcomponent)))
  (return (`local._currentHoveredComponent`) (`local._currentHoveredTarget`)))

(fn `LineTrace`
  (params (ObjectToTrace :type "SceneComponent Object Reference") (Multiplier :type "Float (double-precision)") (TraceChannel :type "ETraceTypeQuery Enum" :default "TraceTypeQuery1") (DrawDebugType :type "EDrawDebugTrace Enum" :default "None"))
  (returns (Output_Get :type "HitResult Structure"))
  (locals (InteractionHit :type "HitResult Structure"))
  (bind _returnvalue (`KismetMathLibrary.GetForwardVector` (`SceneComponent.K2_GetComponentRotation` ObjectToTrace)))
  (bind _returnvalue_2 (+ (`SceneComponent.K2_GetComponentLocation` ObjectToTrace) _returnvalue))
  (bind _outhit (`KismetSystemLibrary.LineTraceSingle` :`Start` _returnvalue_2 :`End` (+ _returnvalue_2 (* _returnvalue Multiplier)) :`TraceChannel` TraceChannel :`DrawDebugType` DrawDebugType :`DrawTime` 2.0))
  (bind _output_get (set `local.InteractionHit` _outhit))
  (return _output_get))

(fn `MultiSphereTrace`
  (params (ObjectToTrace :type "SceneComponent Object Reference") (InteractionMultiplier :type "Float (double-precision)") (SphereMultiplier :type "Float (double-precision)") (DrawDebugType :type "EDrawDebugTrace Enum" :default "None"))
  (returns (Output_Get :type "Array of HitResult Structure"))
  (locals (HitResults :type "Array of HitResult Structure"))
  (bind _returnvalue (`KismetMathLibrary.GetForwardVector` (`SceneComponent.K2_GetComponentRotation` ObjectToTrace)))
  (bind _returnvalue_2 (+ (`SceneComponent.K2_GetComponentLocation` ObjectToTrace) _returnvalue))
  (bind _outhits (`KismetSystemLibrary.SphereTraceMulti` :`Start` _returnvalue_2 :`End` (+ _returnvalue_2 (* _returnvalue InteractionMultiplier)) :`Radius` SphereMultiplier :`TraceChannel` "TraceTypeQuery4" :`DrawDebugType` DrawDebugType :`DrawTime` 1.0))
  (bind _output_get (set `local.HitResults` _outhits))
  (return _output_get))

(fn `SphereTrace`
  (params (ObjectToTrace :type "SceneComponent Object Reference") (InteractionMultiplier :type "Float (double-precision)") (SphereMultiplier :type "Float (double-precision)") (TraceChannel :type "ETraceTypeQuery Enum" :default "TraceTypeQuery1") (DrawDebugType :type "EDrawDebugTrace Enum" :default "None"))
  (returns (Output_Get :type "HitResult Structure"))
  (bind _returnvalue (`KismetMathLibrary.GetForwardVector` (`SceneComponent.K2_GetComponentRotation` ObjectToTrace)))
  (bind _returnvalue_2 (+ (`SceneComponent.K2_GetComponentLocation` ObjectToTrace) _returnvalue))
  (bind _outhit (`KismetSystemLibrary.SphereTraceSingle` :`Start` _returnvalue_2 :`End` (+ _returnvalue_2 (* _returnvalue InteractionMultiplier)) :`Radius` SphereMultiplier :`TraceChannel` TraceChannel :`DrawDebugType` DrawDebugType))
  (return _outhit))
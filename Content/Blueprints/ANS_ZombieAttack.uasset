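; ANS_ZombieAttack is an animation notify that applies a zombie's melee hit during its attack animation.
; When the notify begins on a BP_Zombie, it runs a stationary sphere trace just in front of the actor, with debug drawing enabled.
; If the hit actor implements BPI_Damage, it receives IsDamagableMessage with the zombie's ZombieDamage value.
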(fn `Received_NotifyBegin`
  (params (MeshComp :type "SkeletalMeshComponent Object Reference") (Animation :type "AnimSequenceBase Object Reference") (TotalDuration :type "Float (single-precision)") (EventReference :type "AnimNotifyEventReference Structure (by ref)"))
  (returns (ReturnValue :type Boolean))
  (bind _asbp_zombie (cast `/Game/Blueprints/Zombie/BP_Zombie` (`ActorComponent.GetOwner` MeshComp)))
  (bind _returnvalue (+ (`Actor.K2_GetActorLocation` _asbp_zombie) (* (`Actor.GetActorForwardVector` _asbp_zombie) 100.0)))
  (bind _outhit (`KismetSystemLibrary.SphereTraceSingle` :`WorldContextObject` MeshComp :`Start` _returnvalue :`End` _returnvalue :`Radius` 50.0 :`TraceChannel` "TraceTypeQuery3" :`DrawDebugType` "ForDuration"))
  (bind (_bblockinghit _binitialoverlap _time _distance _location _impactpoint _normal _impactnormal _physmat _hitactor) (`GameplayStatics.BreakHitResult` _outhit))
  (if (`KismetSystemLibrary.DoesImplementInterface` _hitactor "/Game/Blueprints/Weapons/BPI_Damage.BPI_Damage_C")
    (message `/Game/Blueprints/Weapons/BPI_Damage.IsDamagable` _hitactor (`/Game/Blueprints/Zombie/BP_Zombie.ZombieDamage` _asbp_zombie))))
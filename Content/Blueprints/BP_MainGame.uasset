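; Main game logic Blueprint that runs the infection countdown, spawns the zombie manager and restarts the level when the player dies.
; Tick and time damage drain TimeToInfection, updating the HUD through dispatchers and killing the player at zero.
; A looping timer and random stage selection drive stat, weapon and desaturation debuffs, with lore text and debuff-list updates.
; GI_Gamemode saves and restores remaining time across level changes.
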(event `self.ReceiveTick`
  (params (DeltaSeconds :type "Float (single-precision)"))
  (if (not (`self.TimerStopped?`))
    (`self.CountDownTime`)))

(event `self.ReceiveBeginPlay`
  (`|ExecutionSequence`
    (:`then_0`
      ; Manager for Zombies
      (`|SpawnActorFromClass` "/Game/Blueprints/Enemies/DynamicEnemies/BP_DynamicEnemyManager.BP_DynamicEnemyManager_C" (`KismetMathLibrary.MakeTransform` (0.0 0.0 0.0)) "AlwaysSpawn" "MultiplyWithRoot" null null))
    (:`then_1`
      (bind _returnvalue (`GameplayStatics.GetActorOfClass` "/Game/Blueprints/BP_Player.BP_Player_C"))
      (bind _output_get (set `self.Player` _returnvalue))
      (`/Engine/EditorBlueprintResources/StandardMacros.IsValid` _output_get
        (:`Is Valid`
          (add `/Game/Blueprints/BP_Player.UpdTime` _output_get (`|CreateDelegate` :!event `ReceivedTimeDamage`))
          (add `/Game/Blueprints/BP_Player.OnDeath` _output_get (`|CreateDelegate` :!event `PlayerDied`)))))
    (:`then_2`
      (`self.CountDownTxtUpdate` (`self.MaxTimeToInfection`)))))

(event `ReceivedTimeDamage`
  (params (TimeDamage :type "Float (double-precision)"))
  (bind _output_get (set `self.TimeToInfection` (- (`self.TimeToInfection`) TimeDamage)))
  (`self.UpdateHUDTimer` _output_get)
  (`self.CountDownReceivedDamage`))

(event `ChangeLevel`
  (params (LevelText :type Name))
  (bind _asgi_gamemode (cast `/Game/Blueprints/GI_Gamemode` (`GameplayStatics.GetGameInstance`))
    (:`then`
      (`/Game/Blueprints/GI_Gamemode.SaveTime` _asgi_gamemode (`self.TimeToInfection`))
      (`GameplayStatics.OpenLevel` LevelText))
    (:`CastFailed`
      (`KismetSystemLibrary.PrintString` "GameInstanceFailed" :!label _label))))

(event `TimeRanOut`
  (bind _asbp_player (cast `/Game/Blueprints/BP_Player` (`GameplayStatics.GetPlayerCharacter` 0)))
  (`/Game/Blueprints/BP_Player.PlayerDead` _asbp_player))

(event `StartedLevel`
  (bind _asgi_gamemode (cast `/Game/Blueprints/GI_Gamemode` (`GameplayStatics.GetGameInstance`))
    (:`then`
      (`/Game/Blueprints/GI_Gamemode.LoadTime` _asgi_gamemode (`self.TimeToInfection`)))
    (:`CastFailed`
      (goto _label))))

(event `PlayerDied`
  (`/Engine/EditorBlueprintResources/StandardMacros.DoOnce` false
    (:`Completed`
      (`self.CountDownTxtUpdate` 0.0)
      (clear `self.CountDownReceivedDamage`)
      (clear `self.CountDownTxtUpdate`)
      (`GameplayStatics.PlaySound2D` "/Game/Audios/SW_DeathSound.SW_DeathSound" 1.0 1.0 0.0 null null)
      (`PlayerCameraManager.StartCameraFade` :`self` (`GameplayStatics.GetPlayerCameraManager` 0) :`ToAlpha` 1.0 :`Duration` (`self.FadeOutOnDeath`))
      (bind _asgi_gamemode (cast `/Game/Blueprints/GI_Gamemode` (`GameplayStatics.GetGameInstance`)))
      (`/Game/Blueprints/GI_Gamemode.StopMusic` _asgi_gamemode)
      (`KismetSystemLibrary.Delay` (`self.FadeOutOnDeath`))
      (bind _returnvalue (`GameplayStatics.GetCurrentLevelName` true))
      (`GameplayStatics.OpenLevel` (`KismetStringLibrary.Conv_StringToName` _returnvalue)))))

(event `StartTimerEffect`
  (bind _returnvalue (`KismetSystemLibrary.K2_SetTimerDelegate` (`|CreateDelegate` :!event `RandomEventInfection`) (/ (`self.MaxTimeToInfection`) 30) true))
  (set `self.InfectionTimer` _returnvalue))

(event `BWScreen`
  ; BWScrenEffect
  (if (not (`KismetSystemLibrary.K2_IsTimerActiveHandle` (`self.BW Effect`)))
    (bind _returnvalue (`GameplayStatics.GetActorOfClass` "/Script/Engine.PostProcessVolume"))
    (bind (_direction _color) (`Timeline|Timeline` :!via `PlayFromStart`)
      (:`Update`
        (bind (_r _g _b _a) (`KismetMathLibrary.BreakColor` _color))
        (setmembers `PostProcessSettings` :`StructRef` (`PostProcessVolume.Settings` _returnvalue) :`ColorSaturation` (`KismetMathLibrary.MakeVector4` _r _g _b _a)))
      (:`Finished`
        (bind _returnvalue_2 (`KismetSystemLibrary.K2_SetTimerDelegate` (`|CreateDelegate` :!event `BWScreenReset`) 60.0))
        (set `self.BW Effect` _returnvalue_2)))))

(event `BWScreenReset`
  ; BWScrenEffect
  (bind _returnvalue (`GameplayStatics.GetActorOfClass` "/Script/Engine.PostProcessVolume"))
  (bind (_direction _color) (`Timeline|Timeline_0` :!via `ReverseFromEnd`)
    (:`Update`
      (bind (_r _g _b _a) (`KismetMathLibrary.BreakColor` _color))
      (bind _structout (setmembers `PostProcessSettings` :`StructRef` (`PostProcessVolume.Settings` _returnvalue) :`ColorSaturation` (`KismetMathLibrary.MakeVector4` _r _g _b _a)))
      (set `PostProcessVolume.Settings` _structout _returnvalue))))

(fn `AdvanceStage`
  (bind _returnvalue (cast `/Game/Blueprints/Enum/Enum_EfectosPosibles` (`KismetMathLibrary.Conv_IntToByte` (`KismetMathLibrary.RandomInteger` (enumcount `/Game/Blueprints/Enum/Enum_EfectosPosibles`)))))
  (bind _output_get (set `self.LastInfectionStage` (`self.InfectionStage`) :!label _label))
  (if (`|EnumEquality` _output_get _returnvalue)
    (goto _label)
    (else
      (set `self.InfectionStage` _returnvalue)
      (`/Game/Blueprints/BP_Player.ShowBlur` (`self.Player`) (`KismetMathLibrary.RandomFloatInRange` 0.5 1.5)))))

(fn `Black&WhiteEffect`
  (`self.BWScreen`)
  (`/Game/Blueprints/BP_Player.UpdLore` (`self.Player`) "I can't see colors now." 2.0)
  (`self.UpdDebuffList` (`self.InfectionStage`) (`KismetTextLibrary.Conv_StringToText` "Blindness")))

(fn `CountDownTime`
  (bind _output_get (set `self.TimeToInfection` (- (`self.TimeToInfection`) (`GameplayStatics.GetWorldDeltaSeconds`))))
  (`self.UpdateHUDTimer` _output_get))

(fn `MeleeDelay`
  (bind _player (`self.Player`))
  (bind _returnvalue (`self.GetComponentByClass` _player "/Game/Blueprints/Weapons/BP_Weapon_Knife.BP_Weapon_Knife_C"))
  (bind _returnvalue_2 (+ (`self.ReduceSwordAttackTime`) (`/Game/Blueprints/Weapons/BP_Weapon_Knife.MeleeDelay` _returnvalue)))
  (if (<= _returnvalue_2 5.0)
    (set `/Game/Blueprints/Weapons/BP_Weapon_Knife.MeleeDelay` _returnvalue_2 _returnvalue)
    (`/Game/Blueprints/BP_Player.UpdLore` _player "Swinging this sword feels harder now." 2.0)
    (`self.UpdDebuffList` (`self.InfectionStage`) (`|FormatText` "Melee Attack Speed at: {0} seg" _returnvalue_2))))

(fn `PrecitionDecrease1`
  (bind _player (`self.Player`))
  (bind _precitiondecrease (`self.PrecitionDecrease`))
  (bind _precition (`/Game/Blueprints/BP_Player.Precition` _player))
  (set `/Game/Blueprints/BP_Player.Precition` (`KismetMathLibrary.ComposeRotators` _precition _precitiondecrease) _player)
  (`/Game/Blueprints/BP_Player.UpdLore` _player "My hands are trembling." 2.0)
  (`self.UpdDebuffList` (`self.InfectionStage`) (`|FormatText` "Precition Decreased by: {0}%" (`KismetMathLibrary.FClamp` (+ (.yaw _precition) (.yaw _precitiondecrease)) 0.0 100.0))))

(fn `RandomEventInfection`
  (`/Engine/EditorBlueprintResources/StandardMacros.IsValid` (`self.Player`)
    (:`Is Valid`
      (switch `/Game/Blueprints/Enum/Enum_EfectosPosibles` (`self.InfectionStage`)
        (:`NewEnumerator0`
          (`self.SpeedReduction`))
        (:`NewEnumerator3`
          (`self.PrecitionDecrease1`))
        (:`NewEnumerator7`
          (`self.Black&WhiteEffect`))
        (:`NewEnumerator8`
          (`self.SwitchWeaponDelay1`))
        (:`NewEnumerator9`
          (`self.MeleeDelay`)))
      (`self.AdvanceStage`))))

(fn `SpeedReduction`
  (bind _player (`self.Player`))
  (bind _currentweapon (`/Game/Blueprints/BP_Player.CurrentWeapon` _player))
  (bind _returnvalue (- (`/Game/Blueprints/BP_Player.Speed` _player) (`self.SpeedDecrease`)))
  (bind _returnvalue_2 (/ _returnvalue 1.0))
  (if (> _returnvalue 0.5)
    (set `/Game/Blueprints/BP_Player.Speed` _returnvalue_2 _player)
    (bind _output_get (set `/Game/Blueprints/BP_Player.UnderEffect?` true _player))
    (`/Engine/EditorBlueprintResources/StandardMacros.IsValid` _currentweapon
      (:`Is Valid`
        (`/Game/Blueprints/Weapons/BP_Weapon_Master.ChangeAnimation` _currentweapon _output_get))
      (:`Is Not Valid`
        _))
    (`/Game/Blueprints/BP_Player.UpdLore` (`self.Player`) "My legs feel weaker." 2.0)
    (`self.UpdDebuffList` (`self.InfectionStage`) (`|FormatText` "Movement Speed at: {0}%" (* _returnvalue_2 100.0)))))

(fn `SwitchWeaponDelay1`
  (bind _player (`self.Player`))
  (bind _returnvalue (+ (`/Game/Blueprints/BP_Player.TimeToSwitch` _player) (`self.SwitchWeaponDelay`)))
  (if (<= _returnvalue 1.5)
    (set `/Game/Blueprints/BP_Player.TimeToSwitch` _returnvalue _player)
    (`/Game/Blueprints/BP_Player.UpdLore` _player "This weapons are heavy." 2.0)
    (`self.UpdDebuffList` (`self.InfectionStage`) (`|FormatText` "Weapon Swap Speed at: {0}seg" _returnvalue))))

(fn `UpdateHUDTimer`
  (params (Time :type "Float (double-precision)"))
  (bind _returnvalue (`KismetMathLibrary.FClamp` Time 0.0 (`self.MaxTimeToInfection`)))
  (`self.CheckTimeLimit` _returnvalue
    (:`Dead`
      (`self.TimeRanOut`))
    (:`Alive`
      (`self.CountDownTxtUpdate` _returnvalue))))

(fn `UserConstructionScript`)
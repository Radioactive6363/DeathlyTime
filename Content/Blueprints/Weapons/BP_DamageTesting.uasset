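; BP_DamageTesting is a test actor that receives damage and is destroyed when its health runs out.
; Its IsDamagable event subtracts the incoming Damage from Vida, prints the remaining health and damage received as colored Spanish debug messages, then calls Destruido.
; Destruido checks whether Vida is zero or below, and if so prints a destruction message and destroys the actor.
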(event `/Game/Blueprints/Weapons/BPI_Damage.IsDamagable`
  (params (Damage :type "Float (double-precision)") (TypeOfDamage :type "/Game/Blueprints/Enum/E_TypeOfDamage Enum" :default "NewEnumerator0"))
  (bind _output_get (set `self.Vida` (- (`self.Vida`) Damage)))
  (`KismetSystemLibrary.PrintString` (`KismetStringLibrary.Concat_StrStr` "Tengo:  " (`KismetStringLibrary.Conv_DoubleToString` _output_get) " de vida") true true (struct :`R` 0.259266 :`G` 1.0 :`A` 1.0))
  (`KismetSystemLibrary.PrintString` (`KismetStringLibrary.Concat_StrStr` "Recibi: " (`KismetStringLibrary.Conv_DoubleToString` Damage) " de daño!") true true (struct :`R` 1.0 :`G` 0.48018 :`A` 1.0))
  (`self.Destruido`))

(event `Destruido`
  (if (<= (`self.Vida`) 0.0)
    (`KismetSystemLibrary.PrintString` "Fui Destruido!" true true (struct :`R` 1.0 :`B` 0.012164 :`A` 1.0))
    (`self.K2_DestroyActor`)))

(fn `UserConstructionScript`)
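; Zombie character Blueprint that handles running speed, damage and death.
; Incoming damage lowers Life, and at zero or below a one-time Death detaches the controller, disables capsule collision and plays a death animation.
; The mesh switches to ragdoll physics after a short delay, then a timer removes the zombie from BP_ZombieManager's array and destroys it.
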(event `RunningSpeed`
  (set `CharacterMovementComponent.MaxWalkSpeed` (`self.RunningMaxSpeed`) (`self.CharacterMovement`)))

(event `/Game/Blueprints/Weapons/BPI_Damage.IsDamagable`
  (params (Damage :type "Float (double-precision)"))
  (`|ExecutionSequence`
    (:`then_0`
      (`self.DamageReceived` Damage))
    (:`then_1`
      (if (<= (`self.Life`) 0.0)
        (`self.Death`)))))

(event `DamageReceived`
  (params (`DañoRecibido` :type "Float (double-precision)"))
  ; Health Control
  (set `self.Life` (- (`self.Life`) `DañoRecibido`)))

(event `Death`
  ; Comment
  (if (`self.Alive?`)
    (`self.DetachFromControllerPendingDestroy`)
    (set `self.Alive?` false)
    (`SkeletalMeshComponent.PlayAnimation` (`self.Mesh`) (`self.DeathAnimationToPlay`) false)
    (`PrimitiveComponent.SetCollisionEnabled` (`self.CapsuleComponent`) "NoCollision")
    (`KismetSystemLibrary.Delay` 0.5)
    (`PrimitiveComponent.SetSimulatePhysics` (`self.Mesh`) true)
    (`KismetSystemLibrary.K2_SetTimer` null "DestruirZombie" 5.0)))

(event `DestruirZombie`
  (bind _returnvalue (`GameplayStatics.GetActorOfClass` "/Game/Blueprints/Zombie/BP_ZombieManager.BP_ZombieManager_C"))
  (message `/Game/Blueprints/Zombie/BPI_ZombieManagerComm.DeleteZombieFromArray` _returnvalue self)
  (`self.K2_DestroyActor`))

(fn `UserConstructionScript`)
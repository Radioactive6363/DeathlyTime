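; BP_ZombieManager keeps track of live zombie references and relays player detection to all of them.
; Events add zombies to the CurrentZombieCount array and remove them, and CheckLimitOfZombies reports whether its length exactly equals MaxZombieCount.
; On detection, it passes the player to each zombie's AI controller via IAC_Zombie, stopping at the first failed cast.
; CheckLength prints the count for debugging, and MakeArray is an empty stub.
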(event `/Game/Blueprints/Zombie/BPI_ZombieManagerComm.ZombiesSpawned`
  (params (ZombieReference :type "/Game/Blueprints/Zombie/BP_Zombie Object Reference"))
  (`KismetArrayLibrary.Array_Add` (`self.CurrentZombieCount`) ZombieReference))

(event `/Game/Blueprints/Zombie/BPI_ZombieManagerComm.ZombieDetectedPlayer!`
  (params (PlayerReference :type "/Game/Blueprints/BP_Player Object Reference"))
  (for _array_element (`self.CurrentZombieCount`)
    (bind _asiac_zombie (cast `/Game/Blueprints/Zombie/IAC_Zombie` (`AIBlueprintHelperLibrary.GetAIController` _array_element)))
    (`/Game/Blueprints/Zombie/IAC_Zombie.DetectedPlayer` _asiac_zombie PlayerReference)))

(event `/Game/Blueprints/Zombie/BPI_ZombieManagerComm.DeleteZombieFromArray`
  (params (ZombieToDelete :type "/Game/Blueprints/Zombie/BP_Zombie Object Reference"))
  (`/Engine/EditorBlueprintResources/StandardMacros.IsValid` ZombieToDelete
    (:`Is Valid`
      (`KismetArrayLibrary.Array_RemoveItem` (`self.CurrentZombieCount`) ZombieToDelete))))

(event `/Game/Blueprints/Zombie/BPI_ZombieManagerComm.CheckLength`
  (`KismetSystemLibrary.PrintString` (`KismetStringLibrary.Conv_IntToString` (`KismetArrayLibrary.Array_Length` (`self.CurrentZombieCount`)))))

(fn `CheckLimitOfZombies`
  (returns (`isAtLimit?` :type Boolean))
  (return (== (`KismetArrayLibrary.Array_Length` (`self.CurrentZombieCount`)) (`self.MaxZombieCount`))))

(fn `MakeArray`
  (locals (Array :type "Array of /Game/Blueprints/Zombie/BP_Zombie Object Reference")))

(fn `UserConstructionScript`)
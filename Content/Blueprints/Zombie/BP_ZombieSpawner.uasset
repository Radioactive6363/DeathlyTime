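; Zombie spawner actor that places BP_Zombie at random reachable points within a radius, drawn as a debug sphere on construction.
; A spawner type selects looping timers, capped or endless until stopped, or an instant batch followed by self-destruction.
; Each spawn checks BP_ZombieManager's limit, registers there and initializes the AI blackboard.
; All modes except Instant Detected then flag the player as detected, despite that mode's name.
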(event `self.ReceiveBeginPlay`
  (`self.SpawnZombies`))

(event `ContinuousWLimit`
  ; Spawns Zombies Continuosly with Limit
  (if (<= (`self.TempSpawner`) (`self.ZombiesDeseados`))
    (bind _zombieref (`self.SpawnZombie`))
    (`self.DetectedPlayerAlready` _zombieref)
    (`/Engine/EditorBlueprintResources/StandardMacros.IncrementInt` (`self.TempSpawner`))
    (else
      (`KismetSystemLibrary.K2_ClearAndInvalidateTimerHandle` (`self.WithLimit`)))))

(event `SpawnZombies`
  (`KismetSystemLibrary.Delay` 0.2)
  (switch `/Game/Blueprints/Zombie/Enum_TypeOfSpawner` (`self.ZombieSpawnerType`)
    (:`NewEnumerator8`
      ; Spawns Zombies Continuosly with Limit
      (bind _returnvalue (`KismetSystemLibrary.K2_SetTimerDelegate` (delegate `ContinuousWLimit`) (`self.TimeToSpawn`) true))
      (set `self.WithLimit` _returnvalue))
    (:`NewEnumerator0`
      ; Spawns Zombies Continuosly but with NO limit
      (bind _returnvalue_2 (`KismetSystemLibrary.K2_SetTimerDelegate` (delegate `ContinuousNLimit`) (`self.TimeToSpawn`) true))
      (set `self.NoLimit` _returnvalue_2))
    (:`NewEnumerator7`
      ; Spawns Zombies on an Instant Way
      (for _ (range (`self.ZombiesDeseados`))
        (bind _zombieref (`self.SpawnZombie`))
        (`self.DetectedPlayerAlready` _zombieref))
      (`KismetSystemLibrary.Delay` 3.0)
      (`self.K2_DestroyActor`))
    (:`NewEnumerator9`
      ; Spawns Zombies on an Instant Way + AlreadyDetected
      (for _ (range (`self.ZombiesDeseados`))
        (`self.SpawnZombie`))
      (`KismetSystemLibrary.Delay` 3.0)
      (`self.K2_DestroyActor`))))

(event `ContinuousNLimit`
  ; Spawns Zombies Continuosly but with NO limit
  (bind _zombieref (`self.SpawnZombie`))
  (`self.DetectedPlayerAlready` _zombieref))

(event `SetValuesOnBlackBoards`
  (params (ZombieReference :type "Actor Object Reference"))
  ; Set Values On BlackBoard on one zombie
  (bind _asiac_zombie (cast `/Game/Blueprints/Zombie/IAC_Zombie` (`AIBlueprintHelperLibrary.GetAIController` ZombieReference)))
  (`/Game/Blueprints/Zombie/IAC_Zombie.InitializeBlackboard` _asiac_zombie (`self.K2_GetActorLocation`) (`self.SpawnRadius`)))

(event `DetectedPlayerAlready`
  (params (ZombieRef :type "/Game/Blueprints/Zombie/BP_Zombie Object Reference"))
  (bind _asiac_zombie (cast `/Game/Blueprints/Zombie/IAC_Zombie` (`AIBlueprintHelperLibrary.GetAIController` ZombieRef)))
  (`/Game/Blueprints/Zombie/IAC_Zombie.SelfDetectedPlayer` _asiac_zombie))

(event `StopSpawner`
  (`KismetSystemLibrary.K2_ClearAndInvalidateTimerHandle` (`self.WithLimit`))
  (`KismetSystemLibrary.K2_ClearAndInvalidateTimerHandle` (`self.NoLimit`)))

(fn `SpawnZombie`
  (returns (ZombieRef :type "/Game/Blueprints/Zombie/BP_Zombie Object Reference"))
  (bind _returnvalue (`GameplayStatics.GetActorOfClass` "/Game/Blueprints/Zombie/BP_ZombieManager.BP_ZombieManager_C"))
  (bind _isatlimit_ (message `/Game/Blueprints/Zombie/BPI_ZombieManagerComm.CheckLimitOfZombies` _returnvalue))
  (if (not _isatlimit_)
    (bind _returnvalue_2 (`self.ZombieSpawnLocation`))
    (message `/Game/Blueprints/Zombie/BPI_ZombieManagerComm.ZombiesSpawned` _returnvalue _returnvalue_2)
    (`self.SetValuesOnBlackBoards` _returnvalue_2)
    (return _returnvalue_2)))

(fn `UserConstructionScript`
  (`KismetSystemLibrary.DrawDebugSphere` (`self.K2_GetActorLocation`) (`self.SpawnRadius`) 12 (struct :`G` 0.37778 :`B` 1.0 :`A` 0.25) 1.0))

(fn `ZombieSpawnLocation`
  (returns (ReturnValue :type "/Game/Blueprints/Zombie/BP_Zombie Object Reference"))
  (bind (_returnvalue_roll _returnvalue_pitch _returnvalue_yaw) (`KismetMathLibrary.BreakRotator` (`KismetMathLibrary.RandomRotator` true)))
  (bind _returnvalue (`|SpawnActorFromClass` "/Game/Blueprints/Zombie/BP_Zombie.BP_Zombie_C" (`KismetMathLibrary.MakeTransform` (`NavigationSystemV1.K2_GetRandomReachablePointInRadius` (`self.K2_GetActorLocation`) (`self.SpawnRadius`) null null) (`KismetMathLibrary.MakeRotator` 0.0 0.0 _returnvalue_yaw)) "AdjustIfPossibleButDontSpawnIfColliding" "MultiplyWithRoot" null null))
  (return _returnvalue))
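; BP_ZombieSpawner is a one-shot spawner that populates an area with BP_Zombie enemies at BeginPlay, then destroys itself three seconds later.
; Each zombie appears at a random reachable navigation point within SpawnRadius, with random yaw, in a count driven by ZombiesDeseados.
; It passes its location and radius to each zombie's IAC_Zombie AI controller to initialize the blackboard.
; While alive, it draws the radius as a debug sphere every tick.
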(event `self.ReceiveTick`
  (params (DeltaSeconds :type "Float (single-precision)"))
  (`KismetSystemLibrary.DrawDebugSphere` (`self.K2_GetActorLocation`) (`self.SpawnRadius`) 12 (struct :`G` 0.37778 :`B` 1.0 :`A` 0.25)))

(event `self.ReceiveBeginPlay`
  (bind (_returnvalue_roll _returnvalue_pitch _returnvalue_yaw) (`KismetMathLibrary.BreakRotator` (`KismetMathLibrary.RandomRotator` true)))
  (for _ (range (+ (`self.ZombiesDeseados`) 1))
    (bind _returnvalue (`|SpawnActorFromClass` "/Game/BP_Zombie.BP_Zombie_C" (`KismetMathLibrary.MakeTransform` (`NavigationSystemV1.K2_GetRandomReachablePointInRadius` (`self.K2_GetActorLocation`) (`self.SpawnRadius`) null null) (`KismetMathLibrary.MakeRotator` 0.0 0.0 _returnvalue_yaw)) "Undefined" "MultiplyWithRoot" null null))
    (`/Engine/EditorBlueprintResources/StandardMacros.IsValid` _returnvalue
      (:`Is Valid`
        (`self.SetValuesOnBlackBoards` _returnvalue))
      (:`Is Not Valid`
        (`KismetSystemLibrary.PrintString` "Instanciacion NO VALIDA"))))
  (`KismetSystemLibrary.Delay` 3.0)
  (`self.K2_DestroyActor`))

(event `SpawnZombies`)

(event `SetValuesOnBlackBoards`
  (params (ZombieReference :type "Actor Object Reference"))
  (bind _asiac_zombie (cast `/Game/IAC_Zombie` (`AIBlueprintHelperLibrary.GetAIController` ZombieReference))
    (:`then`
      (`/Game/IAC_Zombie.InitializeBlackboard` _asiac_zombie (`self.K2_GetActorLocation`) (`self.SpawnRadius`)))
    (:`CastFailed`
      (`KismetSystemLibrary.PrintString` "Falla Casting de IACZOMBIE"))))

(fn `UserConstructionScript`)
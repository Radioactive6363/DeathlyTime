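; BP_CheatManagerPlayer is a set of debug cheat functions for testing the zombie shooter.
; It toggles player immortality, the weapon component's infinite ammo and instant spawning on every enemy spawner.
; Another cheat tells the enemy manager to remove all zombies, while level cheats restart the current map or open levels by name.
; Targets are found with class lookups at call time, and GoToTestingLevel has its level name set to None.
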(fn `DestroyAllZombies`
  (bind _returnvalue (`GameplayStatics.GetActorOfClass` "/Game/Blueprints/Enemies/DynamicEnemies/BP_DynamicEnemyManager.BP_DynamicEnemyManager_C"))
  (message `/Game/Blueprints/Enemies/DynamicEnemies/BPI_ZombieManagerComm.RemoveAllZombies` _returnvalue)
  (`KismetSystemLibrary.PrintString` "Destroying Zombies"))

(fn `DisableZombieSpawners`
  (bind _outactors (`GameplayStatics.GetAllActorsOfClass` "/Game/Blueprints/Enemies/DynamicEnemies/BP_DynamicEnemySpawner.BP_DynamicEnemySpawner_C"))
  (for _array_element _outactors
    (set `/Game/Blueprints/Enemies/DynamicEnemies/BP_DynamicEnemySpawner.AllowedInstantSpawning?` (not (`/Game/Blueprints/Enemies/DynamicEnemies/BP_DynamicEnemySpawner.AllowedInstantSpawning?` _array_element)) _array_element)))

(fn `GodMode`
  (bind _returnvalue (`GameplayStatics.GetActorOfClass` "/Game/Blueprints/BP_Player.BP_Player_C"))
  (set `/Game/Blueprints/BP_Player.Inmortal?` (not (`/Game/Blueprints/BP_Player.Inmortal?` _returnvalue)) _returnvalue))

(fn `GoToLevel1`
  (locals (LevelName :type Name :default "DT_Level_1"))
  (`GameplayStatics.OpenLevel` (`local.LevelName`)))

(fn `GoToLevel2`
  (locals (LevelName :type Name :default "DT_Level_2"))
  (`GameplayStatics.OpenLevel` (`local.LevelName`)))

(fn `GoToLevel3`
  (locals (LevelName :type Name :default "DT_Blocking_MAP3"))
  (`GameplayStatics.OpenLevel` (`local.LevelName`)))

(fn `GoToTestingLevel`
  (`GameplayStatics.OpenLevel` "None"))

(fn `InfiniteAmmo`
  (bind _returnvalue (`GameplayStatics.GetActorOfClass` "/Game/Blueprints/BP_Player.BP_Player_C"))
  (bind _returnvalue_2 (`Actor.GetComponentByClass` _returnvalue "/Game/Blueprints/Weapons/BP_Weapon_Master.BP_Weapon_Master_C"))
  (`/Engine/EditorBlueprintResources/StandardMacros.IsValid` _returnvalue_2
    (:`Is Valid`
      (bind _output_get (set `/Game/Blueprints/Weapons/BP_Weapon_Master.InfiniteAmmo?` (not (`/Game/Blueprints/Weapons/BP_Weapon_Master.InfiniteAmmo?` _returnvalue_2)) _returnvalue_2))
      (`KismetSystemLibrary.PrintString` (`KismetStringLibrary.Concat_StrStr` "Infinite Ammo " (`KismetStringLibrary.Conv_BoolToString` _output_get))))))

(fn `RestartLevel`
  (bind _returnvalue (`GameplayStatics.GetCurrentLevelName` true))
  (`GameplayStatics.OpenLevel` (`KismetStringLibrary.Conv_StringToName` _returnvalue)))